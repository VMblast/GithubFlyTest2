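; Destructible container transport actor with a shield-based health value, a world-space health bar and an explosion on death.
; DamageHealth subtracts damage, while Tick refreshes the bar, turns it toward the player and, through a short delay, triggers ActorDeath at low health.
; A scene capture is limited to the actor's own components to isolate the mesh, and TargetCameraAim points its spring arm at the player.
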(event `UpdateHealthBar`
  (bind _widget_health (`self.Widget Health`))
  ;[1 1 1] Update Health Bar
  (bind _asbp_container_transport_health (cast `/Game/Container_transport/BP_Container_Transport_Health` (`WidgetComponent.GetUserWidgetObject` (`self.Widget Health`))))
  (`ProgressBar.SetPercent` (`/Game/Container_transport/BP_Container_Transport_Health.ProgressBar_ContainerHealth` _asbp_container_transport_health) (/ (`self.HealthShealds`) 110.0))
  ;[1 1 1] Widget Aim Camera
  (`SceneComponent.K2_SetWorldRotation` _widget_health (`KismetMathLibrary.FindLookAtRotation` (`SceneComponent.K2_GetComponentLocation` _widget_health) (`self.K2_GetActorLocation` (`GameplayStatics.GetPlayerPawn` 0))) false false))

(event `self.ReceiveTick`
  (params (DeltaSeconds :type "Float (single-precision)"))
  ;[1 1 1] Event Tick
  (`|ExecutionSequence`
    (:`then_0`
      ;[1 1 1] Check For Actor Death
      (`KismetSystemLibrary.Delay` 0.2)
      (if (<= (`self.HealthShealds`) 10.0)
        (`self.ActorDeath`)))
    (:`then_1`
      (`self.UpdateHealthBar`))))

(event `ActorDeath`
  ;[1 1 1] Destroy Actor
  (`GameplayStatics.SpawnEmitterAtLocation` "/Game/StarterContent/Particles/P_Explosion_Vehicle.P_Explosion_Vehicle" (`self.K2_GetActorLocation`))
  (`self.K2_DestroyActor`))

(event `TargetCameraAim`
  (bind _springarm (`self.SpringArm`))
  ;[1 1 1] Player Target Aim
  (`SceneComponent.K2_SetWorldRotation` _springarm (`KismetMathLibrary.FindLookAtRotation` (`SceneComponent.K2_GetComponentLocation` _springarm) (`self.K2_GetActorLocation` (`GameplayStatics.GetPlayerPawn` 0))) false false))

(event `DamageHealth`
  ;[1 1 1] Take Damage by Ammount
  (set `self.HealthShealds` (- (`self.HealthShealds`) (`self.DamageAmount`))))

(event `self.ReceiveBeginPlay`
  ;[1 1 1] Isolate Mesh - Mask
  (`SceneCaptureComponent.ShowOnlyActorComponents` (`self.SceneCaptureComponent2D`) (`ActorComponent.GetOwner` (`self.Container_transport`))))

(fn `HealthDisplay`)

(fn `UserConstructionScript`)