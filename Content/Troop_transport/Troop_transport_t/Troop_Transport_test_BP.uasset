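; Test Blueprint for a troop transport that captures an isolated view of its own mesh with a camera that tracks the player.
; On BeginPlay, the SceneCaptureComponent2D show-only list receives the components of the static mesh's owning actor, masking out the rest of the scene.
; Every Tick, TargetCameraAim rotates the SpringArm in world space to look at player pawn 0.
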(event `self.ReceiveBeginPlay`
  ;[1 1 1] Isolate Mesh - Mask
  (`SceneCaptureComponent.ShowOnlyActorComponents` (`self.SceneCaptureComponent2D`) (`ActorComponent.GetOwner` (`self.TroopTransport_Static`))))

(event `self.ReceiveTick`
  (params (DeltaSeconds :type "Float (single-precision)"))
  ;[1 1 1] Event Tick
  (`|ExecutionSequence`
    (:`then_0`
      (`self.TargetCameraAim`))))

(event `TargetCameraAim`
  (bind _springarm (`self.SpringArm`))
  ;[1 1 1] Player Target Aim
  (`SceneComponent.K2_SetWorldRotation` _springarm (`KismetMathLibrary.FindLookAtRotation` (`SceneComponent.K2_GetComponentLocation` _springarm) (`self.K2_GetActorLocation` (`GameplayStatics.GetPlayerPawn` 0))) false false))

(fn `UserConstructionScript`)