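; HUD Blueprint that draws on-screen distance markers over the current objective actors.
; SetObjective stores the actor list, and DrawHUD projects each location, skipping any behind the camera.
; Each visible objective gets a MAT_Markers icon and a label showing player distance in kilometers, offset using measured text width.
; Distance is truncated to two decimals by string splitting; a radar render-target draw is present but never runs.
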(event `/Game/Blueprints/BP_Objective_Marker_Interface.Set Objective`
  (params (Objective :type "Array of Actor Object Reference (by ref)"))
  (set `self.Current Objective` Objective))

(event `self.ReceiveDrawHUD`
  (params (SizeX :type Integer) (SizeY :type Integer))
  (for _array_element (`self.Current Objective`)
    (bind _returnvalue (`self.K2_GetActorLocation` _array_element))
    (bind _y (.y (`self.Project` _returnvalue)))
    (if (> (.z (`self.Project` _returnvalue)) 0.0)
      (bind _returnvalue_2 (`KismetStringLibrary.ParseIntoArray` (`KismetStringLibrary.Conv_DoubleToString` (/ (`KismetMathLibrary.VSize` (- (`self.K2_GetActorLocation` (`GameplayStatics.GetPlayerPawn` 0)) _returnvalue)) 100000.0)) "."))
      (bind _returnvalue_3 (`KismetStringLibrary.Concat_StrStr` "Distance" (`KismetStringLibrary.Concat_StrStr` (`KismetStringLibrary.Concat_StrStr` ": " (`KismetStringLibrary.Concat_StrStr` (`|GetArrayItem` _returnvalue_2) (`KismetStringLibrary.Concat_StrStr` "." (`KismetStringLibrary.GetSubstring` (`|GetArrayItem` _returnvalue_2 1) 0 2)))))))
      (bind _returnvalue_4 (- (.x (`self.Project` _returnvalue)) (/ (`self.GetTextSize` _returnvalue_3 "/Engine/EngineFonts/RobotoDistanceField.RobotoDistanceField") 2.0)))
      (`self.DrawText` _returnvalue_3 (struct :`R` 1.0 :`G` 1.0 :`B` 1.0 :`A` 1.0) (+ _returnvalue_4 16.0) (- _y 60.0) null 1.5)
      (`self.DrawMaterialSimple` "/Game/Markers/MAT_Markers.MAT_Markers" (+ _returnvalue_4 50.0) (- _y 32.0) 32.0 32.0 2.0))))

(fn `UserConstructionScript`)