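; Laser projectile actor that explodes on impact and damages container transports.
; On hit it spawns an explosion effect and a low-pitched hit sound at the impact point, then destroys itself.
; If the hit actor is a Container_transport_BP, it calls that actor's DamageHealth, which takes no damage amount from the laser.
; An older ApplyDamage path with a debug print is discontinued and never runs.
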(event `self.ReceiveHit`
  (params (MyComp :type "PrimitiveComponent Object Reference") (Other :type "Actor Object Reference") (OtherComp :type "PrimitiveComponent Object Reference") (bSelfMoved :type Boolean) (HitLocation :type "Vector Structure") (HitNormal :type "Vector Structure") (NormalImpulse :type "Vector Structure") (Hit :type "HitResult Structure (by ref)"))
  (bind (_bblockinghit _binitialoverlap _time _location _impactpoint) (`GameplayStatics.BreakHitResult` Hit))
  ;[1 1 1] Spawn/Destroy Laser
  (`GameplayStatics.SpawnEmitterAtLocation` "/Game/StarterContent/Particles/P_Explosion.P_Explosion" _impactpoint)
  (`GameplayStatics.PlaySoundAtLocation` "/Game/IP_Fighter/IP_sounds/Laser_hit_Cue.Laser_hit_Cue" _impactpoint (struct) 2.0 0.36)
  (`self.K2_DestroyActor`)
  ;[1 1 1] Damage Health Container Transport
  (bind _ascontainer_transport_bp (cast `/Game/Container_transport/Container_transport_BP` Other))
  (`/Game/Container_transport/Container_transport_BP.DamageHealth` _ascontainer_transport_bp))

(fn `UserConstructionScript`)