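; Outpost D_44 actor that keeps a spring arm aimed at the player and sets up an isolated scene capture of itself.
; On BeginPlay, the scene capture's show-only list is set to the outpost's own components as a mesh mask.
; Every tick, TargetCameraAim sets SpringArm3's world rotation to look at player 0's pawn.
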(event `self.ReceiveTick`
  (params (DeltaSeconds :type "Float (single-precision)"))
  ;[1 1 1] Event Tick
  (`|ExecutionSequence`
    (:`then_0`
      (`self.TargetCameraAim`))))

(event `self.ReceiveBeginPlay`
  ;[1 1 1] Isolate Mesh - Mask
  (`SceneCaptureComponent.ShowOnlyActorComponents` (`self.SceneCaptureComponent2D1`) (`ActorComponent.GetOwner` (`self.Outpost_D_441`))))

(event `TargetCameraAim`
  (bind _springarm3 (`self.SpringArm3`))
  ;[1 1 1] Player Target Aim
  (`SceneComponent.K2_SetWorldRotation` _springarm3 (`KismetMathLibrary.FindLookAtRotation` (`SceneComponent.K2_GetComponentLocation` _springarm3) (`self.K2_GetActorLocation` (`GameplayStatics.GetPlayerPawn` 0))) false false))

(fn `UserConstructionScript`)